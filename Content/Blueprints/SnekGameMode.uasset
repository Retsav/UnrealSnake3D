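; Game mode for a Snek game that handles fruit spawning and game over.
; BeginPlay calls SpawnFruit, which places a Fruit at a fixed height and random XY around the world origin, scaled from the bounds of the first static mesh actor tagged Floor.
; GameOver shows the UI_GameOver widget, pauses the game and switches to UI-only input with a visible cursor.
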(event `self.ReceiveBeginPlay`
  (`self.SpawnFruit`))

(event `GameOver`
  (bind _returnvalue (`|CreateWidget` "/Game/Blueprints/UI_GameOver.UI_GameOver_C" (`GameplayStatics.GetPlayerController` 0)))
  (`UserWidget.AddToViewport` _returnvalue 0)
  (`GameplayStatics.SetGamePaused` true)
  (`WidgetBlueprintLibrary.SetInputMode_UIOnlyEx` (`GameplayStatics.GetPlayerController` 0) _returnvalue)
  (set `PlayerController.bShowMouseCursor` true (`GameplayStatics.GetPlayerController` 0)))

(event `SpawnFruit`
  (bind _outactors (`GameplayStatics.GetAllActorsOfClassWithTag` "/Script/Engine.StaticMeshActor" "Floor"))
  (bind (_origin _boxextent) (`self.GetActorBounds` (`|GetArrayItem` _outactors) false false))
  (bind _returnvalue (/ (.x _boxextent) 2.0))
  (bind _returnvalue_2 (/ (.y _boxextent) 2.0))
  (`|SpawnActorFromClass` "/Game/Blueprints/Fruit.Fruit_C" (`KismetMathLibrary.MakeTransform` (`KismetMathLibrary.MakeVector` (`KismetMathLibrary.RandomFloatInRange` (* _returnvalue -0.8) (* _returnvalue 0.8)) (`KismetMathLibrary.RandomFloatInRange` (* _returnvalue_2 -0.8) (* _returnvalue_2 0.8)) 60.0)) "Undefined" "OverrideRootScale" null null))

(fn `UserConstructionScript`)