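; Player-controlled head of a Snake game that moves one mesh-width every tick in the current direction.
; Directional inputs only turn it when the last movement delta, stored as ActorCurrentLocation, is zero on that axis, preventing reversals.
; Each tick, Tails segments shift into the previous position of the piece ahead.
; AddTail spawns a smaller SnekTail behind the head with the same mesh and appends it to Tails.
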(event `InputAction|MoveUp`
  (params (Key :type "Key Structure"))
  (bind _actorcurrentlocation_x (`KismetMathLibrary.BreakVector` (`self.ActorCurrentLocation`)))
  (:`Pressed`
    (if (== _actorcurrentlocation_x 0.0)
      (set `self.MoveDirection` (1.0 0.0 0.0)))))

(event `InputAction|MoveDown`
  (params (Key :type "Key Structure"))
  (bind _actorcurrentlocation_x (`KismetMathLibrary.BreakVector` (`self.ActorCurrentLocation`)))
  (:`Pressed`
    (if (== _actorcurrentlocation_x 0.0)
      (set `self.MoveDirection` (-1.0 0.0 0.0)))))

(event `InputAction|MoveLeft`
  (params (Key :type "Key Structure"))
  (bind (_actorcurrentlocation_x _actorcurrentlocation_y) (`KismetMathLibrary.BreakVector` (`self.ActorCurrentLocation`)))
  (:`Pressed`
    (if (== _actorcurrentlocation_y 0.0)
      (set `self.MoveDirection` (0.0 -1.0 0.0)))))

(event `InputAction|MoveRight`
  (params (Key :type "Key Structure"))
  (bind (_actorcurrentlocation_x _actorcurrentlocation_y) (`KismetMathLibrary.BreakVector` (`self.ActorCurrentLocation`)))
  (:`Pressed`
    (if (== 0.0 _actorcurrentlocation_y)
      (set `self.MoveDirection` (0.0 1.0 0.0)))))

(event `self.ReceiveBeginPlay`
  (bind _returnvalue (`StaticMesh.GetBoundingBox` (`StaticMeshComponent.StaticMesh` (`self.SnekHead`))))
  (set `self.StepSize` (- (.x (`.Max` (break `Box` _returnvalue))) (.x (break `Box` _returnvalue)))))

(event `self.ReceiveTick`
  (params (DeltaSeconds :type "Float (single-precision)"))
  (set `self.PreviousItemLocation` (`self.K2_GetActorLocation`))
  (`self.K2_AddActorWorldOffset` (* (`self.MoveDirection`) (`self.StepSize`)))
  (set `self.ActorCurrentLocation` (- (`self.K2_GetActorLocation`) (`self.PreviousItemLocation`)))
  (for _array_element (`self.Tails`)
    (bind _output_get (set `self.TailCurrentLocation` (`self.K2_GetActorLocation` _array_element)))
    (`self.K2_SetActorLocation` _array_element (`self.PreviousItemLocation`) false false)
    (set `self.PreviousItemLocation` _output_get)))

(event `AddTail`
  (bind _returnvalue (`|SpawnActorFromClass` "/Game/Blueprints/SnekTail.SnekTail_C" (`KismetMathLibrary.MakeTransform` (- (`self.K2_GetActorLocation`) (* (`self.MoveDirection`) (`self.StepSize`))) (struct) (0.7 0.7 0.7)) "AlwaysSpawn" "OverrideRootScale" null null))
  (`StaticMeshComponent.SetStaticMesh` (`/Game/Blueprints/Trigerable.Mesh` _returnvalue) (`StaticMeshComponent.StaticMesh` (`self.SnekHead`)))
  (`KismetArrayLibrary.Array_Add` (`self.Tails`) _returnvalue))

(fn `UserConstructionScript`)