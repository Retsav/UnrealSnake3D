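; WallDeath is a lethal wall actor for a Snek game that ends the game when the player overlaps it.
; Its PlayerOverlapped event casts the current game mode to SnekGameMode, calls GameOver on it and plays a 2D game-over sound.
; The default BeginPlay, overlap and Tick events are disabled, and the construction script only calls its parent.
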(event `self.PlayerOverlapped`
  (params (Player :type "/Game/Blueprints/BP_SnekHead Object Reference"))
  (bind _assnek_game_mode (cast `/Game/Blueprints/SnekGameMode` (`GameplayStatics.GetGameMode`)))
  (`/Game/Blueprints/SnekGameMode.GameOver` _assnek_game_mode)
  (`GameplayStatics.PlaySound2D` "/Game/SFX/GameOverSFX.GameOverSFX" 1.0 1.0 0.0 null null))

(fn `UserConstructionScript`
  (`parent.UserConstructionScript`))